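; BP_TestGameMode is a test game mode that creates a debug party of characters when play begins.
; After a short delay, BeginPlay creates a party through DRiftGameState, then spawns two PartyCharacterClass actors at a fixed location, names them by index and adds them as members.
; An unconnected debug block that would print the members of party 0 never runs.
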(event EventBeginPlay
  ;[0.75 0.75 0.75 0.5] DEBUG: Creating Test Parties
  (Utilities|FlowControl|Delay 1.0)
  (bind _asdrift_game_state (Utilities|Casting|CastToDRiftGameState (Game|GetGameState)))
  (bind _returnvalue (Class|DRiftGameState|CreateParty _asdrift_game_state))
  (for _index (range 0 1)
    (bind _returnvalue_2 (Game|SpawnActorfromClass (Variables|Default|GetPartyCharacterClass) (Math|Transform|MakeTransform "0.000000,0.000000,90.000000") "AdjustIfPossibleButAlwaysSpawn" "MultiplyWithRoot" 0 0))
    (Class|DRiftPartyCharacter|SetCharacterName _returnvalue_2 (Utilities|String|BuildString(Integer) "Character " "" _index))
    (Class|DRiftGameState|AddMembertoParty _asdrift_game_state _returnvalue _returnvalue_2)))

(event EventTick
  (params (DeltaSeconds :type Float%20%28single-precision%29)))

(fn ConstructionScript)