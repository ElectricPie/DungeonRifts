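; BP_PartyCharacter is a character Blueprint that gives each character a random skeletal mesh as a debug feature.
; On BeginPlay, only the authority picks an entry from DebugRandomMeshs and stores it in SelectedMesh, with separate random rolls for the validity check and assignment.
; The OnRep function for SelectedMesh applies the replicated choice to the Mesh component.
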(event EventBeginPlay
  (bind _debug_randommeshs (Variables|Default|GetDebug_RandomMeshs))
  (bind _debug_randommeshs_2 (Variables|Default|GetDebug_RandomMeshs))
  (bind _returnvalue (Utilities|Array|Length _debug_randommeshs_2))
  (bind _returnvalue_2 (Math|Random|RandomInteger _returnvalue))
  (bind _output (Utilities|Array|Get(acopy) _debug_randommeshs _returnvalue_2))
  ;[0.75 0.75 0.75 0.5] DEBUG: Gives each character a random mesh
  (Networking|SwitchHasAuthority
    (:Authority
      (Utilities|IsValid _output
        (:Is%20Valid
          (Variables|Default|SetSelectedMesh _output))))))

(event Collision|EventActorBeginOverlap
  (params (OtherActor :type Actor%20Object%20Reference)))

(event EventTick
  (params (DeltaSeconds :type Float%20%28single-precision%29)))

(fn ConstructionScript)

(fn OnRepSelectedMesh
  (Components|SkeletalMesh|SetSkeletalMeshAsset (Variables|Character|GetMesh) (Variables|Default|GetSelectedMesh)))